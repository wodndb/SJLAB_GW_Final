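; Interactive descending life line (완강기, emergency escape descender) that the player sets up in stages.
; A trigger box toggles input and shows the current step's widget, while OnInteract advances boolean stages: install hanger, bind rope, hold cylinder, rotate handle via timeline to set AllClear.
; Tick pins cable components and cylinder to the character or throw socket by setting world locations.
; External calls handle cylinder throwing, cable attachment and rope cutting.
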(event OnComponentBeginOverlap(Box)
  (params (OtherActor :type Actor%20Object%20Reference) (OtherComp :type Primitive%20Component%20Object%20Reference) (OtherBodyIndex :type Integer) (bFromSweep :type Boolean) (SweepResult :type Hit%20Result%20Structure%20%28by%20ref%29))
  (bind _returnvalue (Game|GetPlayerCharacter 0))
  ;[1 1 1] 위젯 컨트롤
  (if (Variables|Default|GetallClear)
    (Class|YSmanInterface|CallWidget(Message) _returnvalue "/Game/HUD/W_Wanganggi_All_Clear.W_Wanganggi_All_Clear_C" false)
    (else
      (Input|EnableInput (Game|GetPlayerController 0))
      (if (Variables|Default|GetisHanger)
        (if (Variables|Default|GetLopeBinding)
          (if (Variables|Default|GetSylinder%20on%20Hand)
            (if (Variables|Default|GetisHandleRot)
              (Class|YSmanInterface|CallWidget(Message) _returnvalue "/Game/HUD/W_Wanganggi_All_Clear.W_Wanganggi_All_Clear_C" false)
              (else
                (Class|YSmanInterface|CallWidget(Message) _returnvalue "/Game/HUD/W_Wanganggi_4.W_Wanganggi_4_C" false)))
            (else
              (Class|YSmanInterface|CallWidget(Message) _returnvalue "/Game/HUD/W_Wanganggi_3.W_Wanganggi_3_C" false)))
          (else
            (Class|YSmanInterface|CallWidget(Message) _returnvalue "/Game/HUD/W_Wanganggi_2.W_Wanganggi_2_C" false)))
        (else
          (Class|YSmanInterface|CallWidget(Message) _returnvalue "/Game/HUD/W_Wanganggi_1.W_Wanganggi_1_C" false))))))

(event OnComponentEndOverlap(Box)
  (params (OtherActor :type Actor%20Object%20Reference) (OtherComp :type Primitive%20Component%20Object%20Reference) (OtherBodyIndex :type Integer))
  ;[1 1 1] 위젯 컨트롤
  (if (Variables|Default|GetallClear)
    (Class|YSmanInterface|CallWidget(Message) (Game|GetPlayerCharacter 0) "/Game/HUD/W_Wanganggi_All_Clear.W_Wanganggi_All_Clear_C" false)
    (else
      (Input|DisableInput (Game|GetPlayerController 0)))))

(event EventOnInteract
  (bind _returnvalue (Game|GetPlayerCharacter 0))
  ;[1 1 1] 상호작용
  (if (Variables|Default|GetisHanger) ; 완강기 1단계: 행거 설치
    (if (Variables|Default|GetLopeBinding) ; 완강기 2단계: 줄 연결
      (if (Variables|Default|GetSylinder%20on%20Hand) ; 완강기 3단계: 실린더 쥐기
        (if (not (Variables|Default|GetisHandleRot)) ; 완강기 4단계: 핸들 돌리기
          (bind _handle_rot (Timeline|Rotate%20Handle Play) ; 핸들 돌리기 애니메이션
            (:Update
              (Transformation|SetRelativeRotation (Class|KismetMathLibrary|MakeRot 0.0 _handle_rot 0.0) false)
              (Variables|Default|SetallClear true)
              (Class|YSmanInterface|CallWidget(Message) (Game|GetPlayerCharacter 0) "/Game/HUD/W_Wanganggi_All_Clear.W_Wanganggi_All_Clear_C" false))
            (:Finished
              (Variables|Default|SetisHandleRot true))))
        (else
          (bind _output_boolean (Class|YSmanInterface|GetonHand(Message) _returnvalue))
          (if _output_boolean
            (Class|YSmanInterface|GetHandling(Message) _returnvalue) ; 들고있던거 내리기
          )
          (Variables|Default|SetSylinder%20on%20Hand true)))
      (else
        (Variables|Default|SetLopeBinding true)
        (Rendering|ToggleVisibility false)
        (Class|YSmanInterface|완강기(Message) _returnvalue self)))
    (else
      (Rendering|ToggleVisibility false)
      (Variables|Default|SetisHanger true)
      (Rendering|ToggleVisibility false)
      (Rendering|ToggleVisibility false)
      (Variables|Default|SetisCable true))))

(event EventCableAttachtoGuard
  (params (Socket%20Location :type Vector :default "0, 0, 0"))
  ;[1 1 1] 실린더 던짐
  (Variables|Default|SetCableSetter%20Socket%20Location Socket%20Location)
  (Variables|Default|SetThrowingLope true)
  (Variables|Default|SetSylinder%20on%20Hand false)
  (Components|DestroyComponent)
  (Components|DestroyComponent))

(event EventTick
  (params (DeltaSeconds :type Float%20%28single-precision%29))
  (bind _returnvalue (Game|GetPlayerCharacter 0))
  (bind _cylinder (Variables|Default|GetCylinder))
  (Utilities|FlowControl|Sequence
    (:then_0
      ;[1 1 1] 캐릭터와 연결된 로프 처리
      (if (Variables|Default|GetLopeBinding)
        (if (not (Variables|Default|GetIsCutted))
          (Transformation|SetWorldLocation (Variables|Default|GetCableForCharacter) (+ (Transformation|GetActorLocation (Game|GetPlayerCharacter 0)) "0, 0,10.000000") false)
          (else
            (Components|DestroyComponent)))))
    (:then_1
      ;[1 1 1] 캐릭터 소켓에 실린더 붙이기
      (if (Variables|Default|GetSylinder%20on%20Hand)
        (Collision|SetCollisionEnabled _cylinder "NoCollision")
        (Transformation|SetWorldLocation _cylinder (Transformation|GetSocketLocation _returnvalue "LeftHand") false)
        (Class|YSmanInterface|SetonHand(Message) _returnvalue)))
    (:then_2
      ;[1 1 1] 실린더에 케이블 붙이기
      (if (Variables|Default|GetThrowingLope)
        (Transformation|SetWorldLocation (Variables|Default|GetCable_first) (Variables|Default|GetCableSetter%20Socket%20Location) false)))))

(event EventLopeCut
  (Variables|Default|SetIsCutted true))

(fn ConstructionScript)

(fn CheckAllClear
  (return (Variables|Default|GetallClear)))

(fn GetSylinder
  (Variables|Default|SetisSylinderThrow false)
  (return (Variables|Default|GetCylinder)))

(fn ThrowSylinderOut
  (params (Teleport%20Location :type Vector :default "0, 0, 0") (Socket%20Location :type Vector :default "0, 0, 0"))
  (Variables|Default|SetCableSetter%20Socket%20Location Socket%20Location)
  (Variables|Default|SetSylinder%20on%20Hand false)
  (Transformation|SetRelativeLocation Teleport%20Location false)
  (Class|SceneComponent|DetachfromParent (Variables|Default|GetCable_first) false true)
  (Variables|Default|SetThrowingLope true)
  (return (Transformation|GetWorldLocation (Variables|Default|GetCylinder))))