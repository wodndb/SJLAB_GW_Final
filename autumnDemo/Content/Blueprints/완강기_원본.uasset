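; Interactive descending life line (완강기, an emergency escape descender) that the player sets up step by step.
; An overlap box enables input and shows a prompt widget; each E press advances boolean-tracked stages: hanger, cable, timeline-rotated handle, cylinder throw.
; The final press spawns a Desc_line attached to the player controller and notifies the character.
; Tick keeps the character cable on the pawn until LopeCut triggers a component destroy.
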(event OnComponentBeginOverlap(Box)
  (params (OtherActor :type Actor%20Object%20Reference) (OtherComp :type Primitive%20Component%20Object%20Reference) (OtherBodyIndex :type Integer) (bFromSweep :type Boolean) (SweepResult :type Hit%20Result%20Structure%20%28by%20ref%29))
  (if (not (Variables|Default|GetallClear))
    (Input|EnableInput (Game|GetPlayerController 0))
    (if (not (Variables|Default|GetisHanger))
      (bind _returnvalue (UserInterface|CreateWidget "/Game/HUD/W_Wanganggi_1.W_Wanganggi_1_C"))
      (UserInterface|Viewport|AddtoViewport _returnvalue 0))))

(event OnComponentEndOverlap(Box)
  (params (OtherActor :type Actor%20Object%20Reference) (OtherComp :type Primitive%20Component%20Object%20Reference) (OtherBodyIndex :type Integer))
  (if (not (Variables|Default|GetallClear))
    (Input|DisableInput (Game|GetPlayerController 0))
    (Widget|RemovefromParent (stale OnComponentBeginOverlap(Box) _returnvalue))))

(event Custom|LopeCut
  (Variables|Default|SetIsCutted true))

(event EventTick
  (params (DeltaSeconds :type Float%20%28single-precision%29))
  (if (Variables|Default|GetallClear)
    (if (not (Variables|Default|GetIsCutted))
      (Transformation|SetWorldLocation (Variables|Default|GetCableForCharacter) (+ (Transformation|GetActorLocation (Pawn|GetControlledPawn (Game|GetPlayerController 0))) "0, 0,10.000000") false)
      (else
        (Components|DestroyComponent)))))

(event Input|KeyboardEvents|E
  (bind _returnvalue (Game|GetPlayerController 0))
  (bind _cableforcharacter (Variables|Default|GetCableForCharacter))
  (bind _returnvalue_2 (Pawn|GetControlledPawn _returnvalue))
  (bind _returnvalue_3 (Transformation|GetActorLocation _returnvalue_2))
  (:Pressed
    (if (Variables|Default|GetisHanger)
      (if (Variables|Default|GetisCable)
        (if (Variables|Default|GetisHandleRot)
          (if (Variables|Default|GetisSylinderThrow)
            (Transformation|SetRelativeLocation _cableforcharacter _returnvalue_3 false)
            (Rendering|SetVisibility _cableforcharacter true false)
            (Variables|Default|SetallClear true)
            (bind _returnvalue_4 (Game|SpawnActorfromClass "/Game/Blueprints/desc_line.desc_line_C" (Math|Transform|MakeTransform _returnvalue_3) false 0))
            (Class|Actor|AttachRootComponenttoActor _returnvalue_4 (Game|GetPlayerController 0) "desc_line_socket" "KeepRelativeOffset" true)
            (Class|YSmanInterface|완강기(Message) (Game|GetPlayerCharacter 0) self)
            (else
              (Transformation|SetRelativeLocation (+ (Transformation|GetWorldLocation) "-50.000000,50.000000, 0") false)
              (Variables|Default|SetisSylinderThrow true)))
          (else
            (bind _handle_rot (Timeline|Rotate%20Handle Play)
              (:Update
                (Transformation|SetRelativeRotation (Class|KismetMathLibrary|MakeRot 0.0 _handle_rot 0.0) false))
              (:Finished
                (Variables|Default|SetisHandleRot true)))))
        (else
          (Rendering|ToggleVisibility false)
          (Rendering|ToggleVisibility false)
          (Variables|Default|SetisCable true)))
      (else
        (Rendering|ToggleVisibility false)
        (Variables|Default|SetisHanger true)))))

(fn ConstructionScript)