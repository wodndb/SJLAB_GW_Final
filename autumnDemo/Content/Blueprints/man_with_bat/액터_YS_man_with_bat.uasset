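; Interactive man-with-bat character actor that previews looping skeletal animations when keys are pressed near it.
; The idle animation starts on BeginPlay.
; Trigger box overlaps enable or disable input from the first player controller and toggle two text renders' visibility.
; Number keys play walk, run or idle directly on the skeletal mesh, while key 3 only prints a not-yet-complete message.
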(event OnComponentBeginOverlap(TriggerBox)
  (params (OtherActor :type Actor%20Object%20Reference) (OtherComp :type Primitive%20Component%20Object%20Reference) (OtherBodyIndex :type Integer) (bFromSweep :type Boolean) (SweepResult :type Hit%20Result%20Structure%20%28by%20ref%29))
  ;[1 1 1] 트리거박스 오버랩 이벤트
  (Input|EnableInput (Game|GetPlayerController 0))
  (Rendering|ToggleVisibility (Variables|Default|GetTextRender2) false))

(event OnComponentEndOverlap(TriggerBox)
  (params (OtherActor :type Actor%20Object%20Reference) (OtherComp :type Primitive%20Component%20Object%20Reference) (OtherBodyIndex :type Integer))
  ;[1 1 1] 트리거박스 오버랩 이벤트
  (Input|DisableInput (Game|GetPlayerController 0))
  (Rendering|ToggleVisibility (Variables|Default|GetTextRender2) false))

(event EventBeginPlay
  ;[1 1 1] Begin play
  (Components|Animation|PlayAnimation (Variables|Default|GetSkeletalMesh) "/Game/Animations/man_with_bat/YS_man_with_bat_idle_Anim.YS_man_with_bat_idle_Anim" true))

(event Input|KeyboardEvents|1
  ;[1 1 1] 사용시 동작
  (:Pressed
    (Components|Animation|PlayAnimation (Variables|Default|GetSkeletalMesh) "/Game/Animations/man_with_bat/YS_man_with_bat_walk.YS_man_with_bat_walk" true)))

(event Input|KeyboardEvents|2
  ;[1 1 1] 사용시 동작
  (:Pressed
    (Components|Animation|PlayAnimation (Variables|Default|GetSkeletalMesh) "/Game/Animations/man_with_bat/YS_man_with_bat_run.YS_man_with_bat_run" true)))

(event Input|KeyboardEvents|3
  ;[1 1 1] 사용시 동작
  (:Pressed
    (Development|PrintString "Not compelement yet")))

(event Input|KeyboardEvents|4
  ;[1 1 1] 사용시 동작
  (:Pressed
    (Components|Animation|PlayAnimation (Variables|Default|GetSkeletalMesh) "/Game/Animations/man_with_bat/YS_man_with_bat_idle_Anim.YS_man_with_bat_idle_Anim" true)))

(fn ConstructionScript)