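; Actor for a man with a fire extinguisher whose animations can be previewed with number keys inside a trigger box.
; Entering or leaving the box enables or disables player 0's input and toggles two text renders.
; Keys 1, 2 and 4 loop walk, run and idle animations on the skeletal mesh.
; Key 3 calls montage play on the anim instance, with no montage asset shown.
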(event OnComponentBeginOverlap(TriggerBox)
  (params (OtherActor :type Actor%20Object%20Reference) (OtherComp :type Primitive%20Component%20Object%20Reference) (OtherBodyIndex :type Integer) (bFromSweep :type Boolean) (SweepResult :type Hit%20Result%20Structure%20%28by%20ref%29))
  ;[1 1 1] 트리거박스 오버랩 이벤트
  (Input|EnableInput (Game|GetPlayerController 0))
  (Rendering|ToggleVisibility (Variables|Default|GetTextRender2) false))

(event OnComponentEndOverlap(TriggerBox)
  (params (OtherActor :type Actor%20Object%20Reference) (OtherComp :type Primitive%20Component%20Object%20Reference) (OtherBodyIndex :type Integer))
  ;[1 1 1] 트리거박스 오버랩 이벤트
  (Input|DisableInput (Game|GetPlayerController 0))
  (Rendering|ToggleVisibility (Variables|Default|GetTextRender2) false))

(event Input|KeyboardEvents|1
  ;[1 1 1] 사용시 동작
  (:Pressed
    (Components|Animation|PlayAnimation (Variables|Default|GetSkeletalMesh) "/Game/Animations/man_with_fire_extinguisher/YS_man_with_fire_extinguisher_walk.YS_man_with_fire_extinguisher_walk" true)))

(event Input|KeyboardEvents|2
  ;[1 1 1] 사용시 동작
  (:Pressed
    (Components|Animation|PlayAnimation (Variables|Default|GetSkeletalMesh) "/Game/Animations/man_with_fire_extinguisher/YS_man_with_fire_extinguisher_run.YS_man_with_fire_extinguisher_run" true)))

(event Input|KeyboardEvents|3
  ;[1 1 1] 사용시 동작
  (:Pressed
    (Animation|Montage|MontagePlay (Components|SkeletalMesh|GetAnimInstance (Variables|Default|GetSkeletalMesh)) 0 1.0) ; Play animation on arm mesh
  ))

(event Input|KeyboardEvents|4
  ;[1 1 1] 사용시 동작
  (:Pressed
    (Components|Animation|PlayAnimation (Variables|Default|GetSkeletalMesh) "/Game/Animations/man_with_fire_extinguisher/YS_man_with_fire_extinguisher_idle.YS_man_with_fire_extinguisher_idle" true)))

(fn ConstructionScript)