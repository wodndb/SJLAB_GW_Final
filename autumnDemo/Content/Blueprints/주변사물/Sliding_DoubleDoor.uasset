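; Sliding double door Blueprint that toggles open and closed on the OnInteract event, using a DoorCondition flag.
; BeginPlay caches the relative locations of four static meshes as rest positions.
; Two timelines play or reverse together, each moving one pair of meshes by adding a DoorLocation offset to those positions.
; As wired, each timeline's update reads the other timeline's DoorLocation, and the cached actor location goes unused.
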(event EventBeginPlay
  ;[1 1 1] 문 열고 닫기
  (Variables|Default|Setinitial%20location (Transformation|GetActorLocation))
  (Variables|Default|SetCompInitLoc (Utilities|Array|MakeArray (Variables|/Script/Engine.SceneComponent|GetRelativeLocation (Variables|Default|GetStaticMesh1)) (Variables|/Script/Engine.SceneComponent|GetRelativeLocation (Variables|Default|GetStaticMesh2)) (Variables|/Script/Engine.SceneComponent|GetRelativeLocation (Variables|Default|GetStaticMesh3)) (Variables|/Script/Engine.SceneComponent|GetRelativeLocation (Variables|Default|GetStaticMesh4)))))

(event EventOnInteract
  (bind _compinitloc (Variables|Default|GetCompInitLoc))
  ;[1 1 1] 문 열고 닫기
  (if (Variables|Default|Getdoor_condition)
    (Variables|Default|Setdoor_condition false)
    (Utilities|FlowControl|Sequence
      (:then_0
        (bind _door_location (Timeline|타임라인_0 Play)
          (:Update
            (Utilities|FlowControl|Sequence
              (:then_0
                (Transformation|SetRelativeLocation (Variables|Default|GetStaticMesh1) (+ (stale _door_location_2) (Utilities|Array|Get(acopy) _compinitloc)) false))
              (:then_1
                (Transformation|SetRelativeLocation (Variables|Default|GetStaticMesh2) (+ (stale _door_location_2) (Utilities|Array|Get(acopy) _compinitloc 1)) false))))))
      (:then_1
        (bind _door_location_2 (Timeline|Timeline_0 Play)
          (:Update
            (Utilities|FlowControl|Sequence
              (:then_0
                (Transformation|SetRelativeLocation (Variables|Default|GetStaticMesh3) (+ _door_location (Utilities|Array|Get(acopy) _compinitloc 2)) false))
              (:then_1
                (Transformation|SetRelativeLocation (Variables|Default|GetStaticMesh4) (+ _door_location (Utilities|Array|Get(acopy) _compinitloc 3)) false)))))))
    (else
      (Variables|Default|Setdoor_condition true)
      (Utilities|FlowControl|Sequence
        (:then_0
          (Timeline|타임라인_0 Reverse))
        (:then_1
          (Timeline|Timeline_0 Reverse))))))

(fn ConstructionScript)