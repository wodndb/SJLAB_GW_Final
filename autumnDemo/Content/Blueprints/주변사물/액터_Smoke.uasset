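; Smoke hazard actor that deals gas damage to the player and blocks breathing while they stand inside its box.
; Box overlap sets the damage flag and clears the character's Breath, which returns two seconds after exit.
; While flagged, Tick alternates via DelayingCondition and a one-second Delay between calling CallGasDamage with a new in-smoke widget and removing that widget, pulsing damage about once per second.
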(event OnComponentBeginOverlap(Box)
  (params (OtherActor :type Actor%20Object%20Reference) (OtherComp :type Primitive%20Component%20Object%20Reference) (OtherBodyIndex :type Integer) (bFromSweep :type Boolean) (SweepResult :type Hit%20Result%20Structure%20%28by%20ref%29))
  ;[1 1 1] Overlap 이벤트
  (if (== OtherActor (Game|GetPlayerCharacter 0))
    (bind _as캐릭터_host (Utilities|Casting|CastTo캐릭터_host (Game|GetPlayerCharacter 0)))
    (bind _output_get (Variables|Default|Set캐릭터_Host _as캐릭터_host))
    (Variables|Default|SetDamage true)
    (Variables|/Game/Blueprints/Host/캐릭터_host.캐릭터_host_C|SetBreath _output_get false)))

(event OnComponentEndOverlap(Box)
  (params (OtherActor :type Actor%20Object%20Reference) (OtherComp :type Primitive%20Component%20Object%20Reference) (OtherBodyIndex :type Integer))
  (bind _캐릭터_host (Variables|Default|Get캐릭터_Host))
  ;[1 1 1] Overlap 이벤트
  (if (== (Game|GetPlayerCharacter 0) OtherActor)
    (Variables|Default|SetDamage false)
    (Utilities|FlowControl|Delay 2.0) ; 2초 후 숨쉬기 가능
    (if (not (Variables|/Game/Blueprints/Host/캐릭터_host.캐릭터_host_C|GetBreath _캐릭터_host))
      (Variables|/Game/Blueprints/Host/캐릭터_host.캐릭터_host_C|SetBreath _캐릭터_host true))))

(event EventTick
  (params (DeltaSeconds :type Float%20%28single-precision%29))
  ;[1 1 1] Tick Event
  ;[1 1 1] 초당 데미지
  (if (Variables|Default|GetDamage)
    (if (Variables|Default|GetDelaying%20Condition)
      (Utilities|FlowControl|Delay 1.0)
      (Variables|Default|SetDelaying%20Condition false)
      ;[1 1 1] HUD in Flame for Character
      (Widget|RemovefromParent (stale _returnvalue))
      (else
        (Variables|Default|SetDelaying%20Condition true)
        (Default|CallGasDamage (Variables|Default|Get캐릭터_Host))
        (bind _returnvalue (UserInterface|CreateWidget "/Game/HUD/W_In_Smoke.W_In_Smoke_C" (Game|GetPlayerController 0)))
        (UserInterface|Viewport|AddtoViewport _returnvalue 0)))))

(fn ConstructionScript)

(fn OnRepYSman)