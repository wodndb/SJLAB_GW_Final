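; Stairway smoke hazard that applies gas damage to the player's host character and the child AI character.
; Box and WithChildZone overlaps share logic that stores each character, sets its damage flag and disables Breath.
; Tick uses per-character Delay gates to send gas damage about once a second while alive, also setting a smoke widget on the host.
; On exit, damage stops and Breath returns after a short delay unless the character re-entered.
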(event OnComponentBeginOverlap(withChildZone)
  (params (OtherActor :type Actor%20Object%20Reference) (OtherComp :type Primitive%20Component%20Object%20Reference) (OtherBodyIndex :type Integer) (bFromSweep :type Boolean) (SweepResult :type Hit%20Result%20Structure%20%28by%20ref%29))
  (bind _overlappingactors (Collision|GetOverlappingActors "/Game/Blueprints/Child/캐릭터_child.캐릭터_child_C" :!class /Script/Engine.Actor))
  (bind _item (Utilities|Array|Get(acopy) _overlappingactors))
  ;[1 1 1] Begin Overlap Event
  (Variables|Default|SetOverlapped%20Actor OtherActor)
  (Utilities|FlowControl|Sequence
    (:then_0
      (if (== (Variables|Default|GetOverlapped%20Actor) (Game|GetPlayerCharacter 0))
        (bind _as캐릭터_host (Utilities|Casting|CastTo캐릭터_host (Game|GetPlayerCharacter 0)))
        (bind _output_get (Variables|Default|SetCharacter%20Host _as캐릭터_host))
        (Variables|Default|SetDamage%20to%20Host true)
        (Variables|/Game/Blueprints/Host/캐릭터_host.캐릭터_host_C|SetBreath _output_get false)))
    (:then_1
      (if (== (Variables|Default|GetOverlapped%20Actor) _item)
        (bind _as캐릭터_child (Utilities|Casting|CastTo캐릭터_child _item))
        (bind _output_get_2 (Variables|Default|SetCharacter%20Child _as캐릭터_child))
        (Variables|Default|SetDamage%20to%20Child true)
        (Variables|/Game/Blueprints/Child/캐릭터_child.캐릭터_child_C|SetBreath _output_get_2 false)))))

(event OnComponentEndOverlap(withChildZone)
  (params (OtherActor :type Actor%20Object%20Reference) (OtherComp :type Primitive%20Component%20Object%20Reference) (OtherBodyIndex :type Integer))
  ;[1 1 1] End Overlap Event
  (Variables|Default|SetOverlapped%20Actor OtherActor)
  (Utilities|FlowControl|Sequence
    (:then_0
      (if (== (Variables|Default|GetCharacter%20Host) (Variables|Default|GetOverlapped%20Actor))
        (Variables|Default|SetDamage%20to%20Host false)
        (Utilities|FlowControl|Delay 2.0) ; 2초 후 숨쉬기 가능
        (if (not (Variables|Default|GetDamage%20to%20Host))
          (Variables|/Game/Blueprints/Host/캐릭터_host.캐릭터_host_C|SetBreath (Variables|Default|GetCharacter%20Host) true))))
    (:then_1
      (if (== (Variables|Default|GetOverlapped%20Actor) (Variables|Default|GetCharacter%20Child))
        (Variables|Default|SetDamage%20to%20Child false)
        (Utilities|FlowControl|Delay 2.0) ; 2초 후 숨쉬기 가능
        (if (not (Variables|Default|GetDamage%20to%20Child))
          (Variables|/Game/Blueprints/Child/캐릭터_child.캐릭터_child_C|SetBreath (Variables|Default|GetCharacter%20Child) true))))))

(event OnComponentEndOverlap(Box)
  (params (OtherActor :type Actor%20Object%20Reference) (OtherComp :type Primitive%20Component%20Object%20Reference) (OtherBodyIndex :type Integer))
  ;[1 1 1] End Overlap Event
  (Variables|Default|SetOverlapped%20Actor OtherActor)
  (Utilities|FlowControl|Sequence
    (:then_0
      (if (== (Variables|Default|GetCharacter%20Host) (Variables|Default|GetOverlapped%20Actor))
        (Variables|Default|SetDamage%20to%20Host false)
        (Utilities|FlowControl|Delay 2.0) ; 2초 후 숨쉬기 가능
        (if (not (Variables|Default|GetDamage%20to%20Host))
          (Variables|/Game/Blueprints/Host/캐릭터_host.캐릭터_host_C|SetBreath (Variables|Default|GetCharacter%20Host) true))))
    (:then_1
      (if (== (Variables|Default|GetOverlapped%20Actor) (Variables|Default|GetCharacter%20Child))
        (Variables|Default|SetDamage%20to%20Child false)
        (Utilities|FlowControl|Delay 2.0) ; 2초 후 숨쉬기 가능
        (if (not (Variables|Default|GetDamage%20to%20Child))
          (Variables|/Game/Blueprints/Child/캐릭터_child.캐릭터_child_C|SetBreath (Variables|Default|GetCharacter%20Child) true))))))

(event OnComponentBeginOverlap(Box)
  (params (OtherActor :type Actor%20Object%20Reference) (OtherComp :type Primitive%20Component%20Object%20Reference) (OtherBodyIndex :type Integer) (bFromSweep :type Boolean) (SweepResult :type Hit%20Result%20Structure%20%28by%20ref%29))
  (bind _overlappingactors (Collision|GetOverlappingActors "/Game/Blueprints/Child/캐릭터_child.캐릭터_child_C" :!class /Script/Engine.Actor))
  (bind _item (Utilities|Array|Get(acopy) _overlappingactors))
  ;[1 1 1] Begin Overlap Event
  (Variables|Default|SetOverlapped%20Actor OtherActor)
  (Utilities|FlowControl|Sequence
    (:then_0
      (if (== (Variables|Default|GetOverlapped%20Actor) (Game|GetPlayerCharacter 0))
        (bind _as캐릭터_host (Utilities|Casting|CastTo캐릭터_host (Game|GetPlayerCharacter 0)))
        (bind _output_get (Variables|Default|SetCharacter%20Host _as캐릭터_host))
        (Variables|Default|SetDamage%20to%20Host true)
        (Variables|/Game/Blueprints/Host/캐릭터_host.캐릭터_host_C|SetBreath _output_get false)))
    (:then_1
      (if (== (Variables|Default|GetOverlapped%20Actor) _item)
        (bind _as캐릭터_child (Utilities|Casting|CastTo캐릭터_child _item))
        (bind _output_get_2 (Variables|Default|SetCharacter%20Child _as캐릭터_child))
        (Variables|Default|SetDamage%20to%20Child true)
        (Variables|/Game/Blueprints/Child/캐릭터_child.캐릭터_child_C|SetBreath _output_get_2 false)))))

(event EventTick
  (params (DeltaSeconds :type Float%20%28single-precision%29))
  ;[1 1 1] Tick Event
  (Utilities|FlowControl|Sequence
    (:then_0
      ;[1 1 1] 초당 데미지 - Host
      (if (Variables|Default|GetDamage%20to%20Host)
        (if (Variables|/Game/Blueprints/Host/캐릭터_host.캐릭터_host_C|GetAlive? (Variables|Default|GetCharacter%20Host)) ; 살아있을 때만 데미지를 입힘
          (if (Variables|Default|GetDelaying%20Condition%20for%20Host)
            (Utilities|FlowControl|Delay 1.0)
            (Variables|Default|SetDelaying%20Condition%20for%20Host false)
            (else
              (Variables|Default|SetDelaying%20Condition%20for%20Host true)
              (Class|BPIHost|GasDamage(Message) (Variables|Default|GetCharacter%20Host))
              ;[1 1 1] HUD in Smoke for Character
              (bind _returnvalue (UserInterface|CreateWidget "/Game/HUD/W_In_Smoke.W_In_Smoke_C"))
              (UserInterface|SetWidget (Variables|/Game/Blueprints/Host/캐릭터_host.캐릭터_host_C|GetWidgetEffect_Smoke (Variables|Default|GetCharacter%20Host)) _returnvalue))))))
    (:then_1
      ;[1 1 1] 초당 데미지 - Child
      (if (Variables|Default|GetDamage%20to%20Child)
        (if (Variables|/Game/Blueprints/Child/캐릭터_child.캐릭터_child_C|GetAlive? (Variables|Default|GetCharacter%20Child)) ; 살아있을 때만 데미지를 입힘
          (if (Variables|Default|GetDelaying%20Condition%20for%20Child)
            (Utilities|FlowControl|Delay 1.0)
            (Variables|Default|SetDelaying%20Condition%20for%20Child false)
            (else
              (Variables|Default|SetDelaying%20Condition%20for%20Child true)
              (Class|BPIChild|GasDamage(Message) (Variables|Default|GetCharacter%20Child)))))))))

(fn ConstructionScript)

(fn OnRepYSman)