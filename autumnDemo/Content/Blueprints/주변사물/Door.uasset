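; Interactable door actor that swings open away from or toward either side, depending on which of two trigger boxes was last entered.
; Box overlaps set a side flag, and OnInteract toggles the door, playing one of two yaw timelines and saving that choice so closing reverses the same one.
; Timeline updates set actor yaw as an offset from DoorBody's relative yaw, cached in the construction script.
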(event OnComponentBeginOverlap(Box2)
  (params (OtherActor :type Actor%20Object%20Reference) (OtherComp :type Primitive%20Component%20Object%20Reference) (OtherBodyIndex :type Integer) (bFromSweep :type Boolean) (SweepResult :type Hit%20Result%20Structure%20%28by%20ref%29))
  (Variables|Default|SetLocFromDoor true))

(event OnComponentEndOverlap(Box1)
  (params (OtherActor :type Actor%20Object%20Reference) (OtherComp :type Primitive%20Component%20Object%20Reference) (OtherBodyIndex :type Integer)))

(event OnComponentEndOverlap(Box2)
  (params (OtherActor :type Actor%20Object%20Reference) (OtherComp :type Primitive%20Component%20Object%20Reference) (OtherBodyIndex :type Integer)))

(event OnComponentBeginOverlap(Box1)
  (params (OtherActor :type Actor%20Object%20Reference) (OtherComp :type Primitive%20Component%20Object%20Reference) (OtherBodyIndex :type Integer) (bFromSweep :type Boolean) (SweepResult :type Hit%20Result%20Structure%20%28by%20ref%29))
  (Variables|Default|SetLocFromDoor false))

(event EventOnInteract
  (bind _locfromdoor (Variables|Default|GetLocFromDoor))
  (bind _initrotval (Variables|Default|GetInitRotVal))
  (if (Variables|Default|GetDoorStatus)
    (Variables|Default|SetDoorStatus false)
    (if (Variables|Default|GetOpenedDoorStat)
      (bind _doorrot (Timeline|DoorRotation Reverse)
        (:Update
          (Transformation|SetActorRotation (Class|KismetMathLibrary|MakeRot 0.0 (+ _initrotval _doorrot) 0.0))))
      (else
        (bind _door_rot (Timeline|DoorRotation2 Reverse)
          (:Update
            (Transformation|SetActorRotation (Class|KismetMathLibrary|MakeRot 0.0 (+ _door_rot _initrotval) 0.0))))))
    (else
      (Variables|Default|SetDoorStatus true)
      (Variables|Default|SetOpenedDoorStat _locfromdoor)
      (if _locfromdoor
        (Timeline|DoorRotation Play)
        (else
          (Timeline|DoorRotation2 Play))))))

(fn ConstructionScript
  (Variables|Default|SetInitRotVal (.Yaw (Class|KismetMathLibrary|BreakRot (Variables|/Script/Engine.SceneComponent|GetRelativeRotation (Variables|Default|GetDoorBody))))))