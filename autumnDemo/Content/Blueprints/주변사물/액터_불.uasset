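; Interactable fire actor that the player ignites with E, escalating into an explosion and a burning hazard.
; Trigger box overlap toggles input and the in-flame flag.
; Pressing E runs the small fire (작은불), then after a delay fires the explosion, shockwave impulse and big fire.
; While burning and overlapped, Tick sends heat and negative water through an elemental damage interface to the overlapping actor, spawning an emitter and printing debug text.
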(event OnComponentBeginOverlap(TriggerBox)
  (params (OtherActor :type Actor%20Object%20Reference) (OtherComp :type Primitive%20Component%20Object%20Reference) (OtherBodyIndex :type Integer) (bFromSweep :type Boolean) (SweepResult :type Hit%20Result%20Structure%20%28by%20ref%29))
  ;[1 1 1] 트리거박스 오버랩
  (Input|EnableInput (Game|GetPlayerController 0))
  (Variables|Default|SetInFlame true))

(event OnComponentEndOverlap(TriggerBox)
  (params (OtherActor :type Actor%20Object%20Reference) (OtherComp :type Primitive%20Component%20Object%20Reference) (OtherBodyIndex :type Integer))
  ;[1 1 1] 트리거박스 오버랩
  (Input|DisableInput (Game|GetPlayerController 0))
  (Variables|Default|SetInFlame false))

(event OnComponentHit(TriggerBox)
  (params (OtherActor :type Actor%20Object%20Reference) (OtherComp :type Primitive%20Component%20Object%20Reference) (NormalImpulse :type Vector :default "0, 0, 0") (Hit :type Hit%20Result%20Structure%20%28by%20ref%29))
  (Development|PrintString "Hello"))

(event EventTick
  (params (DeltaSeconds :type Float%20%28single-precision%29))
  ;[1 1 1] 화재발생시 데미지
  (if (and (Variables|Default|GetBurnning) (Variables|Default|GetInFlame))
    (Class|BPIElementalProjectiles|ElementalDamage(Message) (stale OnComponentBeginOverlap(TriggerBox) OtherActor) 0.04 -0.05 0.0) ; Call this interface function on the target blueprint, if it implements it
    (Effects|SpawnEmitteratLocation 0 (Transformation|GetActorLocation (stale OnComponentBeginOverlap(TriggerBox) OtherActor)) "0,0.000000, 0") ; Spawn an impact effect
    (Development|PrintString "Hot!!!!")))

(event Input|KeyboardEvents|E
  (bind _작은_불 (Variables|Default|Get작은%20불))
  (:Pressed
    (Rendering|ToggleVisibility (Variables|Default|GetTextRender) false)
    (Components|Activation|SetActive _작은_불 true false)
    (Utilities|FlowControl|Delay 2.0)
    (Components|Activation|Deactivate _작은_불)
    (Components|Activation|SetActive (Variables|Default|Get폭발) true false)
    (Class|RadialForceComponent|FireImpulse (Variables|Default|Get충격파))
    (Components|Activation|SetActive (Variables|Default|Get큰%20불) true false)
    (Variables|Default|SetBurnning true)))

(fn ConstructionScript)