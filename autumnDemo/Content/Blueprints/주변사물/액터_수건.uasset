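; Towel pickup actor (수건) that swaps the player for a towel-carrying character, provided the player's Heat is zero.
; Its trigger box toggles input and messages the player's W_get_towel prompt widget on entry.
; On interact it gets the player's fire-related properties, handles any held item, and destroys itself and the player.
; It then spawns and possesses 캐릭터_YSman_with_towel near the towel, passing the saved properties on.
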(event OnComponentBeginOverlap(Interactbox)
  (params (OtherActor :type Actor%20Object%20Reference) (OtherComp :type Primitive%20Component%20Object%20Reference) (OtherBodyIndex :type Integer) (bFromSweep :type Boolean) (SweepResult :type Hit%20Result%20Structure%20%28by%20ref%29))
  ;[1 1 1] 트리거박스 오버랩 이벤트
  (Input|EnableInput (Game|GetPlayerController 0))
  (Class|YSmanInterface|CallWidget(Message) (Game|GetPlayerCharacter 0) "/Game/HUD/W_get_towel.W_get_towel_C" false))

(event OnComponentEndOverlap(Interactbox)
  (params (OtherActor :type Actor%20Object%20Reference) (OtherComp :type Primitive%20Component%20Object%20Reference) (OtherBodyIndex :type Integer))
  ;[1 1 1] 트리거박스 오버랩 이벤트
  (Input|DisableInput (Game|GetPlayerController 0)))

(event EventOnInteract
  (bind _returnvalue (Game|GetPlayerCharacter 0))
  (bind _returnvalue_2 (Game|GetPlayerController 0))
  ;[1 1 1] 사용시 동작
  (Class|YSmanInterface|GetProperty(Message) (Game|GetPlayerCharacter 0))
  (if (== (Variables|Default|GetHeat) 0.0)
    (bind _output_boolean (Class|YSmanInterface|GetonHand(Message) _returnvalue))
    (if _output_boolean
      (Class|YSmanInterface|GetHandling(Message) _returnvalue) ; 들고있던거 내리기
    )
    (bind _output_get (Variables|Default|SetPlayer%20Transform (Transformation|GetActorTransform)))
    (bind _output_get_2 (Variables|Default|SetCurrent%20Actor%20Rotation (Transformation|GetActorRotation (Game|GetPlayerCharacter 0))))
    (Actor|DestroyActor self)
    (Pawn|UnPossess _returnvalue_2)
    (Utilities|Casting|CastToPlayerController _returnvalue_2)
    (bind _returnvalue_3 (Game|SpawnActorfromClass "/Game/Blueprints/man_with_towel/캐릭터_YSman_with_towel.캐릭터_YSman_with_towel_C" (Math|Transform|MakeTransform (+ (.Location (Math|Transform|BreakTransform _output_get)) "0,-30.000000,80.000000") (.Rotation (Math|Transform|BreakTransform _output_get)) (.Scale (Math|Transform|BreakTransform _output_get))) true 0))
    (Transformation|SetActorRotation _returnvalue_3 _output_get_2)
    (Pawn|Possess _returnvalue_2 _returnvalue_3)
    (Class|YSmanInterface|SetProperty(Message) (Game|GetPlayerCharacter 0) (Variables|Default|GetHeat) (Variables|Default|Get불에%20대한%20내구성) (Variables|Default|GetWetness) (Variables|Default|GetBurntness) (Variables|Default|Get질식에%20대한%20내구성)) ; 변경된 캐릭터에 속성값 전이
    (else
      (Development|PrintString "You can't take this while burnning!"))))

(event EventSetProperty
  (params (Heat :type Float%20%28single-precision%29) (불에대한내구성 :type Float%20%28single-precision%29) (Wetness :type Float%20%28single-precision%29) (Burntness :type Float%20%28single-precision%29) (질식에대한내구성 :type Float%20%28single-precision%29))
  ;[1 1 1] 캐릭터 속성 받기
  (Variables|Default|SetHeat Heat)
  (Variables|Default|Set불에%20대한%20내구성 불에대한내구성)
  (Variables|Default|SetWetness Wetness)
  (Variables|Default|SetBurntness Burntness)
  (Variables|Default|Set질식에%20대한%20내구성 질식에대한내구성))

(fn ConstructionScript)

(fn OnRepYSman)