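; Sliding door actor that the player opens and closes by interacting while inside its trigger box.
; Box1 overlap events enable and disable input for player controller 0, without checking which actor overlaps.
; OnInteract toggles DoorCondition, playing a timeline forward or, after a short delay, in reverse.
; The timeline moves the whole actor by an offset from the location cached at BeginPlay, without sweep.
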(event OnComponentBeginOverlap(Box1)
  (params (OtherActor :type Actor%20Object%20Reference) (OtherComp :type Primitive%20Component%20Object%20Reference) (OtherBodyIndex :type Integer) (bFromSweep :type Boolean) (SweepResult :type Hit%20Result%20Structure%20%28by%20ref%29))
  ;[1 1 1] Able and Disable input of controller
  (Input|EnableInput (Game|GetPlayerController 0)))

(event OnComponentEndOverlap(Box1)
  (params (OtherActor :type Actor%20Object%20Reference) (OtherComp :type Primitive%20Component%20Object%20Reference) (OtherBodyIndex :type Integer))
  ;[1 1 1] Able and Disable input of controller
  (Input|DisableInput (Game|GetPlayerController 0)))

(event EventBeginPlay
  (Variables|Default|Setinitial%20location (Transformation|GetActorLocation)))

(event EventOnInteract
  (if (Variables|Default|Getdoor_condition)
    (Variables|Default|Setdoor_condition false)
    (bind _door_location (Timeline|타임라인_0 Play)
      (:Update
        (Transformation|SetActorLocation (+ _door_location (Variables|Default|Getinitial%20location)) false)))
    (else
      (Variables|Default|Setdoor_condition true)
      (Utilities|FlowControl|Delay 0.5)
      (Timeline|타임라인_0 Reverse))))

(fn ConstructionScript)