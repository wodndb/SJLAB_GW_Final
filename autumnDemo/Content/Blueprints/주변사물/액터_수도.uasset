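; Water tap actor that lets the player wet a towel they are carrying.
; Overlapping the interact box asks player character 0 whether it has a towel, and if so enables input on the actor and shows the wet-towel widget through a character message.
; Pressing E sets the towel wetness to full via message and calls up the notification widget.
; Leaving the box disables input; the construction script and OnRep_YSman are empty.
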(event OnComponentBeginOverlap(Interactbox)
  (params (OtherActor :type Actor%20Object%20Reference) (OtherComp :type Primitive%20Component%20Object%20Reference) (OtherBodyIndex :type Integer) (bFromSweep :type Boolean) (SweepResult :type Hit%20Result%20Structure%20%28by%20ref%29))
  ;[1 1 1] 트리거박스 오버랩 이벤트
  (bind _have (Class|YSmanInterface|HaveTowel(Message) (Game|GetPlayerCharacter 0)))
  (if _have
    (Input|EnableInput (Game|GetPlayerController 0))
    (Class|YSmanInterface|CallWidget(Message) (Game|GetPlayerCharacter 0) "/Game/HUD/W_wet_towel.W_wet_towel_C" false)))

(event OnComponentEndOverlap(Interactbox)
  (params (OtherActor :type Actor%20Object%20Reference) (OtherComp :type Primitive%20Component%20Object%20Reference) (OtherBodyIndex :type Integer))
  ;[1 1 1] 트리거박스 오버랩 이벤트
  (Input|DisableInput (Game|GetPlayerController 0)))

(event Input|KeyboardEvents|E
  ;[1 1 1] 사용시 동작
  (:Pressed
    (Class|수건인터페이스|SetTowelWetness(Message) (Game|GetPlayerCharacter 0) 1.0)
    (Class|YSmanInterface|CallWidget(Message) (Game|GetPlayerCharacter 0) "/Game/HUD/W_notify_wetTowel.W_notify_wetTowel_C" false)))

(fn ConstructionScript)

(fn OnRepYSman)