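; Smoke hazard actor that spreads across the level and applies gas damage to the player (host) and a child AI.
; After a BeginPlay delay, it sphere-traces along ±X and ±Y and spawns another smoke node in each clear direction, propagating recursively.
; Overlaps on Box or WithChildZone block breathing, restored shortly after exit.
; Tick sends gas damage to living occupants, unthrottled for the host and Delay-throttled for the child.
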(event OnComponentBeginOverlap(withChildZone)
  (params (OtherActor :type Actor%20Object%20Reference) (OtherComp :type Primitive%20Component%20Object%20Reference) (OtherBodyIndex :type Integer) (bFromSweep :type Boolean) (SweepResult :type Hit%20Result%20Structure%20%28by%20ref%29))
  (bind _overlappingactors (Collision|GetOverlappingActors "/Game/Blueprints/Child/캐릭터_child.캐릭터_child_C" :!class /Script/Engine.Actor))
  (bind _item (Utilities|Array|Get(acopy) _overlappingactors))
  ;[1 1 1] Begin Overlap Event
  (Variables|Default|SetOverlapped%20Actor OtherActor)
  (Utilities|FlowControl|Sequence
    (:then_0
      (if (== (Variables|Default|GetOverlapped%20Actor) (Game|GetPlayerCharacter 0))
        (bind _as캐릭터_host (Utilities|Casting|CastTo캐릭터_host (Game|GetPlayerCharacter 0)))
        (bind _output_get (Variables|Default|SetCharacter%20Host _as캐릭터_host))
        (Variables|Default|SetDamage%20to%20Host true)
        (Variables|/Game/Blueprints/Host/캐릭터_host.캐릭터_host_C|SetBreath _output_get false)))
    (:then_1
      (if (== (Variables|Default|GetOverlapped%20Actor) _item)
        (bind _as캐릭터_child (Utilities|Casting|CastTo캐릭터_child _item))
        (bind _output_get_2 (Variables|Default|SetCharacter%20Child _as캐릭터_child))
        (Variables|Default|SetDamage%20to%20Child true)
        (Variables|/Game/Blueprints/Child/캐릭터_child.캐릭터_child_C|SetBreath _output_get_2 false)))))

(event OnComponentEndOverlap(withChildZone)
  (params (OtherActor :type Actor%20Object%20Reference) (OtherComp :type Primitive%20Component%20Object%20Reference) (OtherBodyIndex :type Integer))
  ;[1 1 1] End Overlap Event
  (Variables|Default|SetOverlapped%20Actor OtherActor)
  (Utilities|FlowControl|Sequence
    (:then_0
      (if (== (Variables|Default|GetCharacter%20Host) (Variables|Default|GetOverlapped%20Actor))
        (Variables|Default|SetDamage%20to%20Host false)
        (Utilities|FlowControl|Delay 2.0) ; 2초 후 숨쉬기 가능
        (if (not (Variables|Default|GetDamage%20to%20Host))
          (Variables|/Game/Blueprints/Host/캐릭터_host.캐릭터_host_C|SetBreath (Variables|Default|GetCharacter%20Host) true))))
    (:then_1
      (if (== (Variables|Default|GetOverlapped%20Actor) (Variables|Default|GetCharacter%20Child))
        (Variables|Default|SetDamage%20to%20Child false)
        (Utilities|FlowControl|Delay 2.0) ; 2초 후 숨쉬기 가능
        (if (not (Variables|Default|GetDamage%20to%20Child))
          (Variables|/Game/Blueprints/Child/캐릭터_child.캐릭터_child_C|SetBreath (Variables|Default|GetCharacter%20Child) true))))))

(event OnComponentEndOverlap(Box)
  (params (OtherActor :type Actor%20Object%20Reference) (OtherComp :type Primitive%20Component%20Object%20Reference) (OtherBodyIndex :type Integer))
  ;[1 1 1] End Overlap Event
  (Variables|Default|SetOverlapped%20Actor OtherActor)
  (Utilities|FlowControl|Sequence
    (:then_0
      (if (== (Variables|Default|GetCharacter%20Host) (Variables|Default|GetOverlapped%20Actor))
        (Variables|Default|SetDamage%20to%20Host false)
        (Utilities|FlowControl|Delay 2.0) ; 2초 후 숨쉬기 가능
        (if (not (Variables|Default|GetDamage%20to%20Host))
          (Variables|/Game/Blueprints/Host/캐릭터_host.캐릭터_host_C|SetBreath (Variables|Default|GetCharacter%20Host) true))))
    (:then_1
      (if (== (Variables|Default|GetOverlapped%20Actor) (Variables|Default|GetCharacter%20Child))
        (Variables|Default|SetDamage%20to%20Child false)
        (Utilities|FlowControl|Delay 2.0) ; 2초 후 숨쉬기 가능
        (if (not (Variables|Default|GetDamage%20to%20Child))
          (Variables|/Game/Blueprints/Child/캐릭터_child.캐릭터_child_C|SetBreath (Variables|Default|GetCharacter%20Child) true))))))

(event OnComponentBeginOverlap(Box)
  (params (OtherActor :type Actor%20Object%20Reference) (OtherComp :type Primitive%20Component%20Object%20Reference) (OtherBodyIndex :type Integer) (bFromSweep :type Boolean) (SweepResult :type Hit%20Result%20Structure%20%28by%20ref%29))
  (bind _overlappingactors (Collision|GetOverlappingActors "/Game/Blueprints/Child/캐릭터_child.캐릭터_child_C" :!class /Script/Engine.Actor))
  (bind _item (Utilities|Array|Get(acopy) _overlappingactors))
  ;[1 1 1] Begin Overlap Event
  (Variables|Default|SetOverlapped%20Actor OtherActor)
  (Utilities|FlowControl|Sequence
    (:then_0
      (if (== (Variables|Default|GetOverlapped%20Actor) (Game|GetPlayerCharacter 0))
        (bind _as캐릭터_host (Utilities|Casting|CastTo캐릭터_host (Game|GetPlayerCharacter 0)))
        (bind _output_get (Variables|Default|SetCharacter%20Host _as캐릭터_host))
        (Variables|Default|SetDamage%20to%20Host true)
        (Variables|/Game/Blueprints/Host/캐릭터_host.캐릭터_host_C|SetBreath _output_get false)))
    (:then_1
      (if (== (Variables|Default|GetOverlapped%20Actor) _item)
        (bind _as캐릭터_child (Utilities|Casting|CastTo캐릭터_child _item))
        (bind _output_get_2 (Variables|Default|SetCharacter%20Child _as캐릭터_child))
        (Variables|Default|SetDamage%20to%20Child true)
        (Variables|/Game/Blueprints/Child/캐릭터_child.캐릭터_child_C|SetBreath _output_get_2 false)))))

(event EventBeginPlay
  (bind _self self)
  (bind _self_2 self)
  (bind _self_3 self)
  (bind _self_4 self)
  (bind _returnvalue (Transformation|GetActorLocation _self))
  (bind _returnvalue_2 (Transformation|GetActorLocation _self_2))
  (bind _returnvalue_3 (Transformation|GetActorLocation _self_3))
  (bind _returnvalue_4 (Transformation|GetActorLocation _self_4))
  (bind (_x _y _z) (Math|Vector|BreakVector _returnvalue))
  (bind (_x_2 _y_2 _z_2) (Math|Vector|BreakVector _returnvalue_2))
  (bind (_x_3 _y_3 _z_3) (Math|Vector|BreakVector _returnvalue_3))
  (bind (_x_4 _y_4 _z_4) (Math|Vector|BreakVector _returnvalue_4))
  (bind _returnvalue_5 (- _x_3 2e+02))
  (bind _returnvalue_6 (- _y 2e+02))
  (bind _returnvalue_7 (+ _x_2 2e+02))
  (bind _returnvalue_8 (+ _y_4 2e+02))
  (bind _returnvalue_9 (Math|Vector|MakeVector _x _returnvalue_6 _z))
  (bind _returnvalue_10 (Math|Vector|MakeVector _returnvalue_7 _y_2 _z_2))
  (bind _returnvalue_11 (Math|Vector|MakeVector _returnvalue_5 _y_3 _z_3))
  (bind _returnvalue_12 (Math|Vector|MakeVector _x_4 _returnvalue_8 _z_4))
  (Utilities|FlowControl|Delay 5.0) ; 연기 퍼지는 시간 - 쿨타임
  (Utilities|FlowControl|Sequence
    (:then_0
      ;[1 1 1] +X
      (bind (_outhit _returnvalue_13) (Collision|SphereTraceForObjects _returnvalue_2 _returnvalue_10 (Variables|Default|GetcollisionRadius) (Variables|Default|GetObjectTypeForTrace) false 0 "None"))
      (if (not _returnvalue_13)
        (Game|SpawnActorfromClass "newSmokeNode_C" (Math|Conversions|ToTransform(Vector) _returnvalue_10) false 0 0)))
    (:then_1
      ;[1 1 1] +X
      (bind (_outhit_2 _returnvalue_14) (Collision|SphereTraceForObjects _returnvalue_3 _returnvalue_11 (Variables|Default|GetcollisionRadius) (Variables|Default|GetObjectTypeForTrace) false 0 "None"))
      (if (not _returnvalue_14)
        (Game|SpawnActorfromClass "newSmokeNode_C" (Math|Conversions|ToTransform(Vector) _returnvalue_11) false 0 0)))
    (:then_2
      ;[1 1 1] +X
      (bind (_outhit_3 _returnvalue_15) (Collision|SphereTraceForObjects _returnvalue_4 _returnvalue_12 (Variables|Default|GetcollisionRadius) (Variables|Default|GetObjectTypeForTrace) false 0 "None"))
      (if (not _returnvalue_15)
        (Game|SpawnActorfromClass "newSmokeNode_C" (Math|Conversions|ToTransform(Vector) _returnvalue_12) false 0 0)))
    (:then_3
      ;[1 1 1] +X
      (bind (_outhit_4 _returnvalue_16) (Collision|SphereTraceForObjects _returnvalue _returnvalue_9 (Variables|Default|GetcollisionRadius) (Variables|Default|GetObjectTypeForTrace) false 0 "None"))
      (if (not _returnvalue_16)
        (Game|SpawnActorfromClass "newSmokeNode_C" (Math|Conversions|ToTransform(Vector) _returnvalue_9) false 0 0)))))

(event EventTick
  (params (DeltaSeconds :type Float%20%28single-precision%29))
  ;[1 1 1] Tick Event
  (Utilities|FlowControl|Sequence
    (:then_0
      ;[1 1 1] 초당 데미지 - Host
      (if (Variables|Default|GetDamage%20to%20Host)
        (if (Variables|/Game/Blueprints/Host/캐릭터_host.캐릭터_host_C|GetAlive? (Variables|Default|GetCharacter%20Host)) ; 살아있을 때만 데미지를 입힘
          (Class|BPIHost|GasDamage(Message) (Variables|Default|GetCharacter%20Host)))))
    (:then_1
      ;[1 1 1] 초당 데미지 - Child
      (if (Variables|Default|GetDamage%20to%20Child)
        (if (Variables|/Game/Blueprints/Child/캐릭터_child.캐릭터_child_C|GetAlive? (Variables|Default|GetCharacter%20Child)) ; 살아있을 때만 데미지를 입힘
          (if (Variables|Default|GetDelaying%20Condition%20for%20Child)
            (Utilities|FlowControl|Delay 1.0)
            (Variables|Default|SetDelaying%20Condition%20for%20Child false)
            (else
              (Variables|Default|SetDelaying%20Condition%20for%20Child true)
              (Class|BPIChild|GasDamage(Message) (Variables|Default|GetCharacter%20Child)))))))))

(fn ConstructionScript)

(fn OnRepYSman)