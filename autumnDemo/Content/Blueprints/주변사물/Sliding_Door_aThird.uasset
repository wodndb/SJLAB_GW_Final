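; Sliding door actor that toggles between opening and closing each time OnInteract fires.
; A DoorCondition flag plays or reverses a timeline, whose DoorLocation track offsets StaticMesh1 and StaticMesh2 together from their starting relative locations.
; BeginPlay caches those start positions, along with the actor location and two other meshes' positions, which the movement logic does not use.
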(event EventBeginPlay
  ;[1 1 1] 문 열고 닫기
  (Variables|Default|Setinitial%20location (Transformation|GetActorLocation))
  (Variables|Default|SetCompInitLoc (Utilities|Array|MakeArray (Variables|/Script/Engine.SceneComponent|GetRelativeLocation (Variables|Default|GetStaticMesh1)) (Variables|/Script/Engine.SceneComponent|GetRelativeLocation (Variables|Default|GetStaticMesh2)) (Variables|/Script/Engine.SceneComponent|GetRelativeLocation (Variables|Default|GetStaticMesh3)) (Variables|/Script/Engine.SceneComponent|GetRelativeLocation (Variables|Default|GetStaticMesh4)))))

(event EventOnInteract
  (bind _compinitloc (Variables|Default|GetCompInitLoc))
  ;[1 1 1] 문 열고 닫기
  (if (Variables|Default|Getdoor_condition)
    (Variables|Default|Setdoor_condition false)
    (bind _door_location (Timeline|Timeline_0 Play)
      (:Update
        (Utilities|FlowControl|Sequence
          (:then_0
            (Transformation|SetRelativeLocation (Variables|Default|GetStaticMesh1) (+ _door_location (Utilities|Array|Get(acopy) _compinitloc)) false))
          (:then_1
            (Transformation|SetRelativeLocation (Variables|Default|GetStaticMesh2) (+ _door_location (Utilities|Array|Get(acopy) _compinitloc 1)) false)))))
    (else
      (Variables|Default|Setdoor_condition true)
      (Timeline|Timeline_0 Reverse))))

(fn ConstructionScript)