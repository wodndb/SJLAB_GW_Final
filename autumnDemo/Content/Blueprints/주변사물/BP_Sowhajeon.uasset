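; Fire hydrant (소화전) actor that the player uses to sound the fire alarm in what appears to be a fire-evacuation scenario.
; Its Box overlap enables input and sends the use-prompt widget message, and leaving disables input.
; Interacting records EnableFireplug in the host character's event flags and toggles the alarm.
; Switching on sends a completion widget message and replays the sound through a Delay loop while EnableAlarm stays true.
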(event OnComponentBeginOverlap(Box)
  (params (OtherActor :type Actor%20Object%20Reference) (OtherComp :type Primitive%20Component%20Object%20Reference) (OtherBodyIndex :type Integer) (bFromSweep :type Boolean) (SweepResult :type Hit%20Result%20Structure%20%28by%20ref%29))
  (Input|EnableInput (Game|GetPlayerController 0))
  (Class|YSmanInterface|CallWidget(Message) (Game|GetPlayerCharacter 0) "/Game/HUD/W_use_화재경보기.W_use_화재경보기_C" false))

(event OnComponentEndOverlap(Box)
  (params (OtherActor :type Actor%20Object%20Reference) (OtherComp :type Primitive%20Component%20Object%20Reference) (OtherBodyIndex :type Integer))
  (Input|DisableInput (Game|GetPlayerController 0)))

(event EventOnInteract
  ;[1 1 1] 이벤트 플래그: 소화전 사용
  (bind _as캐릭터_host (Utilities|Casting|CastTo캐릭터_host (Game|GetPlayerCharacter 0)))
  (Variables|/Game/Blueprints/Host/캐릭터_host.캐릭터_host_C|SeteventFlagData _as캐릭터_host (Utilities|Struct|MakeFLAG_eventData (.informFireByShout (Utilities|Struct|BreakFLAG_eventData (Variables|/Game/Blueprints/Host/캐릭터_host.캐릭터_host_C|GeteventFlagData _as캐릭터_host))) true (.reportFireTo119 (Utilities|Struct|BreakFLAG_eventData (Variables|/Game/Blueprints/Host/캐릭터_host.캐릭터_host_C|GeteventFlagData _as캐릭터_host))) (.useFireExCorrect (Utilities|Struct|BreakFLAG_eventData (Variables|/Game/Blueprints/Host/캐릭터_host.캐릭터_host_C|GeteventFlagData _as캐릭터_host))) (.useFireExWithDoor (Utilities|Struct|BreakFLAG_eventData (Variables|/Game/Blueprints/Host/캐릭터_host.캐릭터_host_C|GeteventFlagData _as캐릭터_host))) (.fightSmallFire (Utilities|Struct|BreakFLAG_eventData (Variables|/Game/Blueprints/Host/캐릭터_host.캐릭터_host_C|GeteventFlagData _as캐릭터_host))) (.useWetTowel (Utilities|Struct|BreakFLAG_eventData (Variables|/Game/Blueprints/Host/캐릭터_host.캐릭터_host_C|GeteventFlagData _as캐릭터_host))) (.escapeLowerPose (Utilities|Struct|BreakFLAG_eventData (Variables|/Game/Blueprints/Host/캐릭터_host.캐릭터_host_C|GeteventFlagData _as캐릭터_host))) (.useStair (Utilities|Struct|BreakFLAG_eventData (Variables|/Game/Blueprints/Host/캐릭터_host.캐릭터_host_C|GeteventFlagData _as캐릭터_host))) (.notNearBalcony (Utilities|Struct|BreakFLAG_eventData (Variables|/Game/Blueprints/Host/캐릭터_host.캐릭터_host_C|GeteventFlagData _as캐릭터_host))) (.useELV (Utilities|Struct|BreakFLAG_eventData (Variables|/Game/Blueprints/Host/캐릭터_host.캐릭터_host_C|GeteventFlagData _as캐릭터_host))) (.escapeFrontDoor (Utilities|Struct|BreakFLAG_eventData (Variables|/Game/Blueprints/Host/캐릭터_host.캐릭터_host_C|GeteventFlagData _as캐릭터_host))) (.escapeLooftop (Utilities|Struct|BreakFLAG_eventData (Variables|/Game/Blueprints/Host/캐릭터_host.캐릭터_host_C|GeteventFlagData _as캐릭터_host))) (.escapeGround (Utilities|Struct|BreakFLAG_eventData (Variables|/Game/Blueprints/Host/캐릭터_host.캐릭터_host_C|GeteventFlagData _as캐릭터_host))) (.breakPartition (Utilities|Struct|BreakFLAG_eventData (Variables|/Game/Blueprints/Host/캐릭터_host.캐릭터_host_C|GeteventFlagData _as캐릭터_host))) (.escapeShelter (Utilities|Struct|BreakFLAG_eventData (Variables|/Game/Blueprints/Host/캐릭터_host.캐릭터_host_C|GeteventFlagData _as캐릭터_host))) (.useDescLine (Utilities|Struct|BreakFLAG_eventData (Variables|/Game/Blueprints/Host/캐릭터_host.캐릭터_host_C|GeteventFlagData _as캐릭터_host))) (.useDescLineCorrect (Utilities|Struct|BreakFLAG_eventData (Variables|/Game/Blueprints/Host/캐릭터_host.캐릭터_host_C|GeteventFlagData _as캐릭터_host))) (.NPC_givetowel (Utilities|Struct|BreakFLAG_eventData (Variables|/Game/Blueprints/Host/캐릭터_host.캐릭터_host_C|GeteventFlagData _as캐릭터_host))) (.NPC_guideSafeWay (Utilities|Struct|BreakFLAG_eventData (Variables|/Game/Blueprints/Host/캐릭터_host.캐릭터_host_C|GeteventFlagData _as캐릭터_host))) (.NPC_useEscapeTool (Utilities|Struct|BreakFLAG_eventData (Variables|/Game/Blueprints/Host/캐릭터_host.캐릭터_host_C|GeteventFlagData _as캐릭터_host))) (.awayFromFire (Utilities|Struct|BreakFLAG_eventData (Variables|/Game/Blueprints/Host/캐릭터_host.캐릭터_host_C|GeteventFlagData _as캐릭터_host))) (.behindWind (Utilities|Struct|BreakFLAG_eventData (Variables|/Game/Blueprints/Host/캐릭터_host.캐릭터_host_C|GeteventFlagData _as캐릭터_host)))))
  ;[1 1 1] 소화전 비상벨 재생
  (if (Variables|Default|GetEnableAlarm)
    (Variables|Default|SetEnableAlarm false)
    (else
      (Class|YSmanInterface|CallWidget(Message) (Game|GetPlayerCharacter 0) "/Game/HUD/W_화재경보기_complete.W_화재경보기_complete_C" false)
      (Variables|Default|SetEnableAlarm true)
      (Audio|PlaySoundatLocation "/Game/Sound/S_Fire_Alarm.S_Fire_Alarm" (Variables|/Script/Engine.SceneComponent|GetRelativeLocation (Variables|Default|GetCube)) :!label _label)
      (Utilities|FlowControl|Delay 11.5)
      (if (Variables|Default|GetEnableAlarm)
        (goto _label)))))

(fn ConstructionScript)