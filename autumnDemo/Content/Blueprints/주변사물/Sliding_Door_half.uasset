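; Interactable half-height sliding door that the player can open, close and, while open, jump through to the other side.
; OnInteract toggles DoorCondition and plays or reverses a timeline that offsets two of the meshes from their cached relative positions.
; Box1 overlap enables input and sends the open or close widget message to the player character.
; Two side volumes track the player's side, so F teleports them to the opposite marker and calls DropMessage.
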(event OnComponentBeginOverlap(Box1)
  (params (OtherActor :type Actor%20Object%20Reference) (OtherComp :type Primitive%20Component%20Object%20Reference) (OtherBodyIndex :type Integer) (bFromSweep :type Boolean) (SweepResult :type Hit%20Result%20Structure%20%28by%20ref%29))
  (bind _returnvalue (Game|GetPlayerCharacter 0))
  ;[1 1 1] Able and Disable input of controller
  (Input|EnableInput (Game|GetPlayerController 0))
  (if (Variables|Default|Getdoor_condition)
    (Class|YSmanInterface|CallWidget(Message) _returnvalue "/Game/HUD/W_open_door.W_open_door_C" false) ; 문열기 출력
    (else
      (Class|YSmanInterface|CallWidget(Message) _returnvalue "/Game/HUD/W_close_door.W_close_door_C" false) ; 문닫기 출력
    )))

(event OnComponentEndOverlap(Box1)
  (params (OtherActor :type Actor%20Object%20Reference) (OtherComp :type Primitive%20Component%20Object%20Reference) (OtherBodyIndex :type Integer))
  ;[1 1 1] Able and Disable input of controller
  (Input|DisableInput (Game|GetPlayerController 0)))

(event OnComponentBeginOverlap(A_Location)
  (params (OtherActor :type Actor%20Object%20Reference) (OtherComp :type Primitive%20Component%20Object%20Reference) (OtherBodyIndex :type Integer) (bFromSweep :type Boolean) (SweepResult :type Hit%20Result%20Structure%20%28by%20ref%29))
  ;[1 1 1] 구역설정
  (Variables|Default|SetInA_Location true)
  (Variables|Default|SetInB_Location false))

(event OnComponentEndOverlap(A_Location)
  (params (OtherActor :type Actor%20Object%20Reference) (OtherComp :type Primitive%20Component%20Object%20Reference) (OtherBodyIndex :type Integer))
  ;[1 1 1] 구역설정
  (Variables|Default|SetInA_Location false)
  (Variables|Default|SetInB_Location false))

(event OnComponentEndOverlap(B_Location)
  (params (OtherActor :type Actor%20Object%20Reference) (OtherComp :type Primitive%20Component%20Object%20Reference) (OtherBodyIndex :type Integer))
  ;[1 1 1] 구역설정
  (Variables|Default|SetInA_Location false)
  (Variables|Default|SetInB_Location false))

(event OnComponentBeginOverlap(B_Location)
  (params (OtherActor :type Actor%20Object%20Reference) (OtherComp :type Primitive%20Component%20Object%20Reference) (OtherBodyIndex :type Integer) (bFromSweep :type Boolean) (SweepResult :type Hit%20Result%20Structure%20%28by%20ref%29))
  ;[1 1 1] 구역설정
  (Variables|Default|SetInA_Location false)
  (Variables|Default|SetInB_Location true))

(event EventBeginPlay
  (Variables|Default|Setinitial%20location (Transformation|GetActorLocation))
  (Variables|Default|SetCompInitLoc (Utilities|Array|MakeArray (Variables|/Script/Engine.SceneComponent|GetRelativeLocation (Variables|Default|GetStaticMesh1)) (Variables|/Script/Engine.SceneComponent|GetRelativeLocation (Variables|Default|GetStaticMesh2)) (Variables|/Script/Engine.SceneComponent|GetRelativeLocation (Variables|Default|GetStaticMesh3)) (Variables|/Script/Engine.SceneComponent|GetRelativeLocation (Variables|Default|GetStaticMesh4)))))

(event EventOnInteract
  (bind _compinitloc (Variables|Default|GetCompInitLoc))
  (if (Variables|Default|Getdoor_condition)
    (Variables|Default|Setdoor_condition false)
    (bind _door_location (Timeline|Timeline_0 Play)
      (:Update
        (Utilities|FlowControl|Sequence
          (:then_0
            (Transformation|SetRelativeLocation (Variables|Default|GetStaticMesh3) (+ _door_location (Utilities|Array|Get(acopy) _compinitloc 2)) false))
          (:then_1
            (Transformation|SetRelativeLocation (Variables|Default|GetStaticMesh4) (+ _door_location (Utilities|Array|Get(acopy) _compinitloc 3)) false)))))
    (else
      (Variables|Default|Setdoor_condition true)
      (Timeline|Timeline_0 Reverse))))

(event Input|KeyboardEvents|F
  (bind _returnvalue (Game|GetPlayerCharacter 0))
  (bind _returnvalue_2 (Game|GetPlayerCharacter 0))
  ;[1 1 1] 뛰어내리기
  (:Pressed
    (if (not (Variables|Default|Getdoor_condition)) ; 문이 열려있을 때만 작동
      (if (Variables|Default|GetInA_Location)
        (Transformation|SetActorLocation _returnvalue_2 (Transformation|GetWorldLocation (Variables|Default|GetB_Location)) false)
        (Class|YSmanInterface|Drop(Message) _returnvalue_2)
        (elif (Variables|Default|GetInB_Location)
          (Transformation|SetActorLocation _returnvalue (Transformation|GetWorldLocation (Variables|Default|GetA_Location)) false)
          (Class|YSmanInterface|Drop(Message) _returnvalue))))))

(fn ConstructionScript)