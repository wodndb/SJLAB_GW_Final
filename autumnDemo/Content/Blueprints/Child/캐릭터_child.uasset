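; AI child character in a fire-evacuation game that accompanies the Host and can take its towel, throw a cylinder and yield.
; Overlap with the Host's WithChildZone toggles blackboard-driven following and movement, notifies the Host and copies its stance on entry.
; Fire damages life; gas drains oxygen, more slowly with a wet towel, then life.
; The fail event shows a widget and returns to the menu.
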(event OnComponentBeginOverlap(CapsuleComponent)
  (params (OtherActor :type Actor%20Object%20Reference) (OtherComp :type Primitive%20Component%20Object%20Reference) (OtherBodyIndex :type Integer) (bFromSweep :type Boolean) (SweepResult :type Hit%20Result%20Structure%20%28by%20ref%29))
  (bind _character_host (Variables|Default|GetCharacter%20Host))
  ;[1 1 1] Host와 함께 있는지 없는지를 확인하고 자신의 정보를 Host에 알림
  (bind (_boolean _host) (CallFunction|IsOverlappedHost? OtherActor OtherComp))
  (if _boolean
    (bind _output_get (Variables|Default|Setwith%20Host true))
    (CallFunction|MoveOn/Off true) ; 움직일 수 있게 함
    (CallFunction|SetFollowerandSetCharacterHost _host)
    (AI|Components|Blackboard|SetValueasBool (AI|GetBlackboard self) (Utilities|Name|MakeLiteralName "with Host") _output_get)
    (Class|BPIHost|SetChild(Message) _character_host self)
    (Class|BPIHost|IsHostwithChild?(Message) _character_host true)
    ;[1 1 1] Host 동작 따라하기
    (if (Variables|/Game/Blueprints/Host/캐릭터_host.캐릭터_host_C|GetPose%20Low%20Stance (Variables|Default|GetCharacter%20Host)) ; Host의 동작을 따라한다
      (CallFunction|LetDown)
      (else
        (CallFunction|LetUp)))))

(event OnComponentEndOverlap(CapsuleComponent)
  (params (OtherActor :type Actor%20Object%20Reference) (OtherComp :type Primitive%20Component%20Object%20Reference) (OtherBodyIndex :type Integer))
  ;[1 1 1] Host와 함께 있는지 없는지를 확인하고 자신의 정보를 Host에 알림
  (bind _boolean (CallFunction|IsOverlappedHost? OtherActor OtherComp))
  (if _boolean
    (bind _output_get (Variables|Default|Setwith%20Host false))
    (CallFunction|MoveOn/Off false) ; 움직일 수 없게 함
    (AI|Components|Blackboard|SetValueasBool (AI|GetBlackboard self) (Utilities|Name|MakeLiteralName "with Host") _output_get)
    (Class|BPIHost|IsHostwithChild?(Message) (Variables|Default|GetCharacter%20Host) false)
    ;[1 1 1] "어린이와 함께 있지 않습니다." 위젯 생성
    (bind _returnvalue (UserInterface|CreateWidget "/Game/HUD/W_Not_with_Child.W_Not_with_Child_C"))
    (UserInterface|SetWidget (Variables|/Game/Blueprints/Host/캐릭터_host.캐릭터_host_C|GetWidgetNotify (Variables|Default|GetCharacter%20Host)) _returnvalue)))

(event Custom|Fail_Event
  ;[1 1 1] Fail Event
  (bind _returnvalue (UserInterface|CreateWidget "/Game/HUD/W_Child_Fail.W_Child_Fail_C"))
  (UserInterface|SetWidget (Variables|/Game/Blueprints/Host/캐릭터_host.캐릭터_host_C|GetWidgetNotify (Variables|Default|GetCharacter%20Host)) _returnvalue)
  (Utilities|FlowControl|Delay 3.0)
  (Game|OpenLevel(byName) "SPRING_MENU") ; 위젯을 띄우고 3초후 메뉴로 이동합니다.
)

(event EventGasDamage
  ;[1 1 1] Fire Damage and Gas Damage Event
  (if (> (Variables|Default|GetOxygen%20Gage) 0)
    (if (Variables|Default|Gethave%20Wet%20Towel)
      (Variables|Default|SetOxygen%20Gage (- (Variables|Default|GetOxygen%20Gage) 5))
      (else
        (Variables|Default|SetOxygen%20Gage (- (Variables|Default|GetOxygen%20Gage) 10))))
    (else
      (Variables|Default|SetOxygen%20Gage 0)
      (Variables|Default|SetLife%20Gage (- (Variables|Default|GetLife%20Gage) 10))
      (CallFunction|CheckAlive))))

(event EventFireDamage
  ;[1 1 1] Fire Damage and Gas Damage Event
  (Variables|Default|SetLife%20Gage (- (Variables|Default|GetLife%20Gage) 10))
  (CallFunction|CheckAlive))

(event EventLetDown
  ;[1 1 1] Up / Down Pose and Character Speed
  (Variables|Default|SetPose%20Low%20Stance true)
  (Variables|/Script/Engine.CharacterMovementComponent|SetMaxWalkSpeed (Variables|Character|GetCharacterMovement) 1.5e+02))

(event EventLetUp
  ;[1 1 1] Up / Down Pose and Character Speed
  (Variables|Default|SetPose%20Low%20Stance false)
  (Variables|/Script/Engine.CharacterMovementComponent|SetMaxWalkSpeed (Variables|Character|GetCharacterMovement) 2e+02))

(event EventCanIMove?
  (params (boolean :type Boolean))
  ;[1 1 1] 움직일 수 있는지를 설정
  (AI|Components|Blackboard|SetValueasBool (AI|GetBlackboard self) (Utilities|Name|MakeLiteralName "Can I Move?") boolean))

(event EventDetachTowel
  ;[1 1 1] 수건 내리기
  (if (Variables|Default|Gethave%20Towel)
    (Actor|DestroyActor (Variables|Default|GetSpawned%20Towel))
    (Game|SpawnActorfromClass "/Game/Blueprints/주변사물/수건/액터_HangingTowel.액터_HangingTowel_C" (Math|Conversions|ToTransform(Vector) (Math|Transform|TransformLocation (Transformation|GetActorTransform (Game|GetPlayerCharacter 0)) "30.000000,40.000000,-90.000000")) true 0 0)
    (Variables|Default|Sethave%20Wet%20Towel false)
    (Variables|Default|Sethave%20Towel false)))

(event EventTowel
  (params (Is%20wet? :type Boolean))
  (bind _character_host (Variables|Default|GetCharacter%20Host))
  ;[1 1 1] 수건 받기
  (if (Variables|/Game/Blueprints/Host/캐릭터_host.캐릭터_host_C|Gethave%20Towel (Variables|Default|GetCharacter%20Host)) ; Host가 수건을 가지고 있을 때만 동작
    (Variables|/Game/Blueprints/Host/캐릭터_host.캐릭터_host_C|Sethave%20Wet%20Towel _character_host false)
    (Variables|/Game/Blueprints/Host/캐릭터_host.캐릭터_host_C|Sethave%20Towel _character_host false)
    (Class|Actor|DetachRootComponentfromParent (Variables|/Game/Blueprints/Host/캐릭터_host.캐릭터_host_C|GetSpawned%20Towel _character_host) true) ; Host에서 떼서 Child에 붙이기
    (bind _output_get (Variables|Default|SetSpawned%20Towel (Variables|/Game/Blueprints/Host/캐릭터_host.캐릭터_host_C|GetSpawned%20Towel _character_host)))
    (Class|Actor|AttachRootComponentto _output_get (Variables|Character|GetMesh) "RH Towel Socket" "SnapToTarget" true)
    (Variables|Default|Sethave%20Towel true)
    (Variables|Default|Sethave%20Wet%20Towel Is%20wet?)))

(event EventDoYield
  (bind _returnvalue (Utilities|Name|MakeLiteralName "Yield"))
  (bind _self self)
  (bind _returnvalue_2 (AI|GetBlackboard _self))
  ;[1 1 1] Yield
  (bind _returnvalue_3 (Game|SpawnActorfromClass "/Game/Blueprints/Target.Target_C" (Transformation|GetWorldTransform (Variables|/Game/Blueprints/Host/캐릭터_host.캐릭터_host_C|GetForward%20Target (Variables|Default|GetCharacter%20Host))) true 0 0))
  (Actor|SetLifeSpan _returnvalue_3 1.0)
  (AI|Components|Blackboard|SetValueasObject (AI|GetBlackboard self) (Utilities|Name|MakeLiteralName "Backward") _returnvalue_3)
  (AI|Components|Blackboard|SetValueasBool _returnvalue_2 _returnvalue true) ; Yield On
  (Utilities|FlowControl|Delay 2.0)
  (AI|Components|Blackboard|SetValueasBool _returnvalue_2 _returnvalue false) ; Yield Off
)

(event EventThrowCylinder
  (params (Cable :type Cable%20Component%20Object%20Reference))
  ;[1 1 1] Throw Cylinder
  (bind _projectile_transform_to_use (CallFunction|ThrowingCylinderTrace (Transformation|GetWorldLocation (Variables|Default|GetThrowing%20Cylinder%20Spot))))
  (bind _returnvalue (Game|SpawnActorfromClass "/Game/Blueprints/주변사물/완강기/액터_Projectile_Cylinder.액터_Projectile_Cylinder_C" _projectile_transform_to_use true 0 0))
  (Class|CableComponent|SetAttachEndto Cable _returnvalue "Cable Attach Spot") ; 케이블을 새로 생성된 던져지는 실린더에 재연결
)

(event EventTick
  (params (DeltaSeconds :type Float%20%28single-precision%29))
  ;[1 1 1] 초당 숨차기
  (if (and (Variables|Default|GetBreath) (< (Variables|Default|GetOxygen%20Gage) 50)) ; 숨을 쉴 수 있는 상태이고, 산소량이 최대치보다 낮을 때만 동작
    (if (Variables|Default|GetDelaying%20Condition)
      (Utilities|FlowControl|Delay 1.0)
      (Variables|Default|SetDelaying%20Condition false)
      (else
        (Variables|Default|SetDelaying%20Condition true)
        (bind _output_get (Variables|Default|SetOxygen%20Gage (+ (Variables|Default|GetOxygen%20Gage) 5)))))))

(event EventOnInteract
  ;[0 1 0.03529] 플레이어와 최초 상호작용 (인터페이스) -> 선택지 생성
  (Class|BPIHost|TelltoChild(Message) (Variables|Default|GetCharacter%20Host)))

(fn ConstructionScript
  (bind _asw_hpbar_child (Utilities|Casting|CastToW_HPbar_child (UserInterface|GetUserWidgetObject (Variables|Default|GetWidget))))
  (Variables|/Game/HUD/W_HPbar_child.W_HPbar_child_C|SetCharacterData _asw_hpbar_child self))

(fn CheckAlive
  (if (<= (Variables|Default|GetLife%20Gage) 0)
    (Variables|Default|SetAlive? false)
    (CallFunction|FailEvent)))

(fn ThrowingCylinderTrace
  (params (Projectile%20Origin :type Vector))
  (bind _cylinder_hand (Variables|Default|GetCylinder%20hand))
  (bind _returnvalue (Transformation|GetWorldLocation _cylinder_hand))
  (bind _returnvalue_2 (Math|Vector|GetForwardVector _cylinder_hand))
  (bind _returnvalue_3 (* _returnvalue_2 5e+03))
  (bind _returnvalue_4 (+ _returnvalue _returnvalue_3))
  (bind (_outhit _returnvalue_5) (Collision|LineTraceForObjects _returnvalue _returnvalue_4 (Utilities|Array|MakeArray "ObjectTypeQuery1" "ObjectTypeQuery2") false 0 "None")) ; Trace forwards 10000 units in the direction the player is aiming
  (return (Math|Transform|MakeTransform Projectile%20Origin (Math|Rotator|FindLookatRotation Projectile%20Origin (Math|Vector|SelectVector (.Location (Collision|BreakHitResult _outhit)) _returnvalue_4 _returnvalue_5)))))

(fn SetFollowerandSetCharacterHost
  (params (Character%20Host :type 캐릭터%20Host%20Object%20Reference))
  (AI|Components|Blackboard|SetValueasObject (AI|GetBlackboard self) (Utilities|Name|MakeLiteralName "Follower") Character%20Host)
  (Variables|Default|SetCharacter%20Host Character%20Host))

(fn IsOverlappedHost?
  (params (Overlapped%20Actor :type Actor%20Object%20Reference) (Overlapped%20Component :type Primitive%20Component%20Object%20Reference))
  (bind _as캐릭터_host (Utilities|Casting|CastTo캐릭터_host Overlapped%20Actor)
    (:then
      (LocalVariables|Setbool%20State (== (Variables|/Game/Blueprints/Host/캐릭터_host.캐릭터_host_C|Getwith%20Child%20Zone _as캐릭터_host) Overlapped%20Component)))
    (:CastFailed
      (LocalVariables|Setbool%20State false)))
  (return (LocalVariables|Getbool%20State) _as캐릭터_host))

(fn MoveOn/Off
  (params (boolean :type Boolean))
  (CallFunction|CanIMove? boolean))