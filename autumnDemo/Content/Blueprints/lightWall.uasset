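; Breakable lightweight partition wall built on a destructible component.
; Overlapping its interact box passes the partition-breaking widget to the player character's widget message call.
; A hit on the destructible disables its collision and the collision box's, fires a radial force impulse, then destroys the component after a short delay.
; The construction script stores the arrow's relative location as the initial location.
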(event OnComponentHit(Destructible1)
  (params (OtherActor :type Actor%20Object%20Reference) (OtherComp :type Primitive%20Component%20Object%20Reference) (NormalImpulse :type Vector :default "0, 0, 0") (Hit :type Hit%20Result%20Structure%20%28by%20ref%29))
  (bind _destructible1 (Variables|Default|GetDestructible1))
  (Collision|SetCollisionEnabled (Variables|Default|GetCollision%20Box) "NoCollision")
  (Class|RadialForceComponent|FireImpulse (Variables|Default|GetRadialForce1))
  (Collision|SetCollisionEnabled _destructible1 "NoCollision")
  (Utilities|FlowControl|Delay 2.5)
  (Components|DestroyComponent _destructible1))

(event OnComponentBeginOverlap(InteractBox)
  (params (OtherActor :type Actor%20Object%20Reference) (OtherComp :type Primitive%20Component%20Object%20Reference) (OtherBodyIndex :type Integer) (bFromSweep :type Boolean) (SweepResult :type Hit%20Result%20Structure%20%28by%20ref%29))
  (Class|YSmanInterface|CallWidget(Message) (Game|GetPlayerCharacter 0) "/Game/HUD/W_경량칸막이부수기.W_경량칸막이부수기_C" false))

(fn ConstructionScript
  (Variables|Default|SetInitialLocation (Variables|/Script/Engine.SceneComponent|GetRelativeLocation (Variables|Default|GetArrow1))))