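; BPC_Host is a human Blueprint, derived from a parent class, that adds zoom-camera facing and fire hazard screen effects.
; While the zoom camera is on, a mouse-input event turns the actor to the control rotation's pitch and yaw, with roll removed.
; Separate flame and smoke events create their HUD widgets and assign them to the matching effect widget components.
; The child BeginPlay hook is empty and the construction script only calls the parent.
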(event EventBeginPlayforChildClass
  ;[1 1 1] Begin Play Event
)

(event EventHUDinFlame
  ;[0.9578 0.9553 1] HUD in Flame
  (bind _returnvalue (UserInterface|CreateWidget "/Game/HUD/W_In_Flame.W_In_Flame_C"))
  (UserInterface|SetWidget (Variables|Default|GetWidgetEffect_Flame) _returnvalue))

(event EventHUDinSmoke
  ;[1 1 1] HUD in Smoke
  (bind _returnvalue (UserInterface|CreateWidget "/Game/HUD/W_In_Smoke.W_In_Smoke_C"))
  (UserInterface|SetWidget (Variables|Default|GetWidgetEffect_Smoke) _returnvalue))

(event EventSetActorRotationwithMouseInput
  (bind _returnvalue (Pawn|GetControlRotation :!class /Script/Engine.Pawn))
  (bind (_pitch _yaw) (Class|KismetMathLibrary|BreakRot _returnvalue))
  ;[1 1 1] Zoom Camera 시점 변환
  (if (Variables|Default|GetZoom%20Camera%20On)
    (Transformation|SetActorRotation (Math|Conversions|RotationFromXVector (Math|Vector|GetForwardVector (Class|KismetMathLibrary|MakeRot _pitch _yaw 0.0))))))

(fn ConstructionScript
  (|CallParentFunction))